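; GStreamer source actor pairing a scene capture with a GstPipeline and GstAppSrc component.
; Its construction script passes the pipeline name, config and autostart to the pipeline and binds the app source by the same name.
; BeginPlay creates the capture's render target at runtime and optionally previews it on a cube through a dynamic material.
; Tick writes real time in seconds to a text render.
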(event `self.ReceiveBeginPlay`
  (bind _drawrt (`self.DrawRT`))
  (bind _returnvalue (`KismetRenderingLibrary.CreateRenderTarget2D` (`self.TextureWidth`) (`self.TextureHeight`) (`self.TextureFormat`)))
  (set `SceneCaptureComponent2D.TextureTarget` _returnvalue (`self.SceneCapture`))
  (`SceneComponent.SetVisibility` (`self.Cube`) _drawrt false)
  (if _drawrt
    (bind _returnvalue_2 (`KismetMaterialLibrary.CreateDynamicMaterialInstance` "/Game/GStreamer/MAT_TexturePreview.MAT_TexturePreview"))
    (`MaterialInstanceDynamic.SetTextureParameterValue` _returnvalue_2 "Texture" (`SceneCaptureComponent2D.TextureTarget` (`self.SceneCapture`)))
    (`PrimitiveComponent.SetMaterial` (`self.Cube`) 0 _returnvalue_2)))

(event `self.ReceiveTick`
  (params (DeltaSeconds :type "Float (single-precision)"))
  (`TextRenderComponent.K2_SetText` (`self.TextRender`) (`KismetTextLibrary.Conv_DoubleToText` (`GameplayStatics.GetRealTimeSeconds`) "HalfToEven" false true 1 324 1 1)))

(fn `UserConstructionScript`
  (bind _gstpipeline (`self.GstPipeline`))
  (set `GstPipelineComponent.PipelineName` (`self.PipelineName`) _gstpipeline)
  (set `GstPipelineComponent.PipelineConfig` (`self.PipelineConfig`) _gstpipeline)
  (set `GstPipelineComponent.PipelineAutostart` (`self.Autostart`) _gstpipeline)
  (set `GstAppSrcComponent.PipelineName` (`self.PipelineName`) (`self.GstAppSrc`)))